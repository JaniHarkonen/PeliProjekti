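; CollectibleStar is a scrolling pickup that the player collects for points.
; Each tick it moves by Speed scaled by global time dilation, not delta seconds.
; Overlap with the living Hero, matched by object name, plays a sound and calls EdPointsCollected.
; The same actor is recycled near InitialPosition with random X/Z offset after collection or after passing the negative X limit.
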(event OnComponentHit(RenderComponent)
  (params (HitComponent :type Primitive%20Component%20Object%20Reference) (OtherActor :type Actor%20Object%20Reference) (OtherComp :type Primitive%20Component%20Object%20Reference) (NormalImpulse :type Vector :default "0, 0, 0") (Hit :type Hit%20Result%20Structure%20%28by%20ref%29)))

(event EventBeginPlay)

(event Collision|EventActorBeginOverlap
  (params (OtherActor :type Actor%20Object%20Reference))
  (bind _returnvalue (Math|Random|RandomFloatinRange -5e+01 5e+01))
  ;[1 1 1] Kun törmätään pelaajaan
  ;;[1 1 1] Toteutetaan törmäyskoodi vain, jos pelaaja ei ole kuollut
  (bind _ashero (Utilities|Casting|CastToHero (Game|GetPlayerCharacter 0)))
  (if (Variables|/Game/Blueprints/Hero.Hero_C|GetplayerIsAlive _ashero)
    (if (Utilities|Enum|Equal(Enum) (Utilities|GetObjectName OtherActor) (Utilities|GetObjectName (Game|GetPlayerCharacter 0)))
      (Audio|PlaySound2D "/Game/Sounds/sndCollect.sndCollect" 1.0 1.0 0.0 0 0)
      (Default|CallEdPointsCollected)
      (Transformation|SetActorLocation (+ (Variables|Default|GetinitialPosition) (Math|Vector|MakeVector _returnvalue 0.0 _returnvalue)) false false))))

(event EventTick
  (params (DeltaSeconds :type Float%20%28single-precision%29))
  (bind _returnvalue (Math|Random|RandomFloatinRange -5e+01 5e+01))
  (Transformation|AddActorWorldOffset (* (Variables|Default|Getspeed) (Class|GameplayStatics|GetGlobalTimeDilation)))
  ;[1 1 1] Kun esine on liukunut pois ruudulta
  (if (< (.X (Math|Vector|BreakVector (Transformation|GetActorLocation))) -1e+03)
    (Transformation|SetActorLocation (+ (Variables|Default|GetinitialPosition) (Math|Vector|MakeVector _returnvalue 0.0 _returnvalue)) false false)))

(fn ConstructionScript)