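; Player-controlled 2D hero character that moves along the world X axis and jumps through input axes.
; BeginPlay switches to game-only input and marks the player alive.
; Tick freezes the sprite animation while falling and clamps X between MinX and MaxX to keep the hero on the level.
; Space toggles pause by flipping global time dilation between stopped and normal.
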(event EventBeginPlay
  (Input|SetInputModeGameOnly (Game|GetPlayerController 0))
  (Variables|Default|SetplayerIsAlive true))

(event Collision|EventActorBeginOverlap
  (params (OtherActor :type Actor%20Object%20Reference)))

(event EventTick
  (params (DeltaSeconds :type Float%20%28single-precision%29))
  (bind _returnvalue (Transformation|GetActorLocation))
  (bind _sprite (Variables|Default|GetSprite))
  (bind (_x _y _z) (Math|Vector|BreakVector _returnvalue))
  ;[1 1 1] Pysäytä animaatio, kun hahmo on ilmassa
  (if (AI|Components|NavMovement|IsFalling (Variables|Character|GetCharacterMovement))
    (Components|Timeline|SetPlayRate _sprite 0.0)
    (else
      (Components|Timeline|SetPlayRate _sprite 2.0)))
  ;[1 1 1] Rajoitetaan pelaajan liikkuvuutta x-akselilla, jottei pelaaja tipu kentältä
  (Transformation|SetActorLocation (Math|Vector|MakeVector (Math|Float|Clamp(Float) _x (Variables|Default|GetminX) (Variables|Default|GetmaxX)) _y _z) false false))

(event Input|AxisEvents|InputAxisJump
  (params (AxisValue :type Float%20%28single-precision%29))
  (if (not (Math|Float|NearlyEqual(Float) AxisValue 0.0 1e-06))
    (Character|Jump)))

(event Input|AxisEvents|InputAxisMove_right
  (params (AxisValue :type Float%20%28single-precision%29))
  (Pawn|Input|AddMovementInput "1.000000, 0, 0" AxisValue false))

(event Input|AxisEvents|InputAxisMove_left
  (params (AxisValue :type Float%20%28single-precision%29))
  (Pawn|Input|AddMovementInput "-1.000000, 0, 0" AxisValue false))

(event Input|KeyboardEvents|SpaceBar
  (params (Key :type Key%20Structure))
  ;[1 1 1] Paussi
  (:Pressed
    (if (== (Class|GameplayStatics|GetGlobalTimeDilation) 1.0)
      (Utilities|Time|SetGlobalTimeDilation 0.0)
      (else
        (Utilities|Time|SetGlobalTimeDilation 1.0)))))

(fn ConstructionScript)